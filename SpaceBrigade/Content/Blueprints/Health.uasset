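; Health pickup actor that restores a fixed amount of player health on overlap, then destroys itself.
; When an actor tagged "player" overlaps, it adds to PlayerHealth on MainGameState2, capped at the maximum, and plays a collect sound.
; Tick spins it by a fixed yaw step per frame and bobs it vertically using a sine delta.
; The particle burst and delayed-destroy logic are disconnected and never run.
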(event EventBeginPlay)

(event Collision|EventActorBeginOverlap
  (params (OtherActor :type Actor%20Object%20Reference))
  ;[1 1 1] Check if overlapping with player. If so, update player health and remove. If player health would end up being greater than 100 after collision, then make sure health does not exceed 100
  (if (Actor|ActorHasTag OtherActor "player")
    (bind _asmain_game_state_2 (Utilities|Casting|CastToMainGameState2 (Game|GetGameState)))
    (if (> (+ (Variables|/Game/GameModes/MainGameState2.MainGameState2_C|GetPlayerHealth _asmain_game_state_2) 3e+01) 1e+02)
      (Variables|/Game/GameModes/MainGameState2.MainGameState2_C|SetPlayerHealth _asmain_game_state_2 1e+02)
      (Audio|PlaySoundatLocation "/Game/Sounds/CollectSound.CollectSound" (Transformation|GetActorLocation) "0, 0, 0" 1.0 1.0 0.0 0 0 0)
      (else
        (Variables|/Game/GameModes/MainGameState2.MainGameState2_C|SetPlayerHealth _asmain_game_state_2 (+ (Variables|/Game/GameModes/MainGameState2.MainGameState2_C|GetPlayerHealth _asmain_game_state_2) 3e+01))
        (Audio|PlaySoundatLocation "/Game/Sounds/CollectSound.CollectSound" (Transformation|GetActorLocation) "0, 0, 0" 1.0 1.0 0.0 0 0 0)))
    (Actor|DestroyActor)))

(event EventTick
  (params (DeltaSeconds :type Float%20%28single-precision%29))
  (bind _returnvalue (Transformation|GetActorRotation))
  (bind _returnvalue_2 (Transformation|GetActorLocation))
  (bind _returnvalue_3 (Actor|GetGameTimeSinceCreation))
  (bind (_x _y _z) (Math|Vector|BreakVector _returnvalue_2))
  (bind (_roll _pitch _yaw) (Math|Rotator|BreakRotator _returnvalue))
  ;[1 1 1] Move the health up and down using sin function every tick
  (Transformation|SetActorRotation (Math|Rotator|MakeRotator _roll _pitch (+ _yaw 1.0)))
  (Transformation|SetActorLocation (Math|Vector|MakeVector _x _y (+ _z (* (- (Math|Trig|Sin(Radians) (+ _returnvalue_3 DeltaSeconds)) (Math|Trig|Sin(Radians) _returnvalue_3)) 8e+01))) false false)
  (if (Variables|Default|Getwaiting)
    (Variables|Default|Setwait (- (Variables|Default|Getwait) 1))))

(fn ConstructionScript)