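; Player spaceship that flies continuously along its local Z, with smoothed yaw and pitch steering, clamped thrust and bullet firing.
; Axis inputs update speeds that Tick applies as local movement and rotation; the roll-banking logic is unconnected.
; Tick reads health from the level-specific game state to toggle two damage smoke effects.
; Overlapping a planet-tagged actor plays destruction effects, returns the ship to origin, removes a life and restores health.
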(event EventBeginPlay)

(event Collision|EventActorBeginOverlap
  (params (OtherActor :type Actor%20Object%20Reference))
  (bind _returnvalue (Game|GetGameState))
  ;[1 1 1] check if player collides with planet. Decrease lives and respawn
  (if (Actor|ActorHasTag OtherActor "planet")
    (Effects|SpawnEmitteratLocation "/Game/Particles/DestroyParticle.DestroyParticle" (Transformation|GetActorLocation) "0, 0, 0" "5.000000,5.000000,5.000000")
    (Audio|PlaySoundatLocation "/Game/Sounds/DestroySound.DestroySound" (Transformation|GetActorLocation (Game|Player|GetPlayerPawn 0)) "0, 0, 0" 1.0 1.0 0.0 0 0 0)
    (if (<= (Variables|Default|GetWait) 0)
      _
      (else
        (while (> (Variables|Default|GetWait) 0)
          (Variables|Default|SetWait (- (Variables|Default|GetWait) 1)))))
    (Variables|Default|SetWait 80)
    (Transformation|SetActorLocation "0, 0, 0" false false)
    (bind _returnvalue_2 (Game|GetCurrentLevelName true))
    (if (Utilities|Enum|Equal(Enum) _returnvalue_2 "Level1")
      (bind _asmain_game_state (Utilities|Casting|CastToMainGameState _returnvalue))
      (Variables|/Game/GameModes/MainGameState.MainGameState_C|SetLives _asmain_game_state (- (Variables|/Game/GameModes/MainGameState.MainGameState_C|GetLives _asmain_game_state) 1))
      (Variables|/Game/GameModes/MainGameState.MainGameState_C|SetPlayerHealth _asmain_game_state 1e+02)
      (else
        (bind _asmain_game_state_2 (Utilities|Casting|CastToMainGameState2 _returnvalue))
        (Variables|/Game/GameModes/MainGameState2.MainGameState2_C|SetLives _asmain_game_state_2 (- (Variables|/Game/GameModes/MainGameState2.MainGameState2_C|GetLives _asmain_game_state_2) 1))
        (Variables|/Game/GameModes/MainGameState2.MainGameState2_C|SetPlayerHealth _asmain_game_state_2 1e+02)))))

(event EventTick
  (params (DeltaSeconds :type Float%20%28single-precision%29))
  (bind _returnvalue (Game|GetGameState))
  (bind _returnvalue_2 (Utilities|Time|GetWorldDeltaSeconds))
  ;[1 1 1] Tick - Move player ship every frame, set smoke particles to active or not active if player health reaches certain threshold
  (Variables|Default|SetDeltaTime DeltaSeconds)
  (Transformation|AddActorLocalOffset (Math|Vector|MakeVector 0.0 0.0 (* (* DeltaSeconds 2.0) (Variables|Default|GetCurrentPlayerSpeed))) false false)
  (Transformation|AddActorLocalRotation (Math|Rotator|MakeRotator (* _returnvalue_2 (Variables|Default|GetCurrentRollSpeed)) (* _returnvalue_2 (Variables|Default|GetCurrentPitchSpeed)) (* _returnvalue_2 (Variables|Default|GetCurrentYawSpeed))) false false)
  (bind _returnvalue_3 (Game|GetCurrentLevelName true))
  (if (Utilities|Enum|Equal(Enum) _returnvalue_3 "Level1")
    (bind _asmain_game_state (Utilities|Casting|CastToMainGameState _returnvalue))
    (if (<= (Variables|/Game/GameModes/MainGameState.MainGameState_C|GetPlayerHealth _asmain_game_state) 5e+01)
      (Components|Activation|SetActive (Variables|Default|GetSmokeParticle) true false)
      (if (<= (Variables|/Game/GameModes/MainGameState.MainGameState_C|GetPlayerHealth _asmain_game_state) 3e+01)
        (Components|Activation|SetActive (Variables|Default|GetSmokeParticle2) true false))
      (else
        (Components|Activation|SetActive (Variables|Default|GetSmokeParticle) false false)
        (Components|Activation|SetActive (Variables|Default|GetSmokeParticle2) false false)))
    (else
      (bind _asmain_game_state_2 (Utilities|Casting|CastToMainGameState2 _returnvalue))
      (if (<= (Variables|/Game/GameModes/MainGameState2.MainGameState2_C|GetPlayerHealth _asmain_game_state_2) 5e+01)
        (Components|Activation|SetActive (Variables|Default|GetSmokeParticle) true false)
        (if (<= (Variables|/Game/GameModes/MainGameState2.MainGameState2_C|GetPlayerHealth _asmain_game_state_2) 3e+01)
          (Components|Activation|SetActive (Variables|Default|GetSmokeParticle2) true false))
        (else
          (Components|Activation|SetActive (Variables|Default|GetSmokeParticle) false false)
          (Components|Activation|SetActive (Variables|Default|GetSmokeParticle2) false false))))))

(event Input|ActionEvents|InputActionShoot
  (params (Key :type Key%20Structure :default "None"))
  ;[1 1 1] Shoot a bullet when space bar pressed
  (:Pressed
    (Game|SpawnActorfromClass "/Game/Blueprints/Bullet_Blueprint.Bullet_Blueprint_C" (Math|Transform|ComposeTransforms (Math|Transform|MakeTransform "0, 0,190.000000" "0, 0, 0" "0.600000,0.600000,0.600000") (Transformation|GetActorTransform)) "Undefined" 0 0)
    (Audio|PlaySoundatLocation "/Game/Sounds/ShootSound.ShootSound" (Transformation|GetActorLocation) "0, 0, 0" 1.0 1.0 0.0 0 0 0)))

(event Input|AxisEvents|InputAxisHorizontal
  (params (AxisValue :type Float%20%28single-precision%29))
  ;[1 1 1] Move player ship left and right from input
  (Variables|Default|SetCurrentYawSpeed (Math|Interpolation|FInterpTo (Variables|Default|GetCurrentYawSpeed) (* AxisValue (Variables|Default|GetPlayerTurnSpeed)) (Utilities|Time|GetWorldDeltaSeconds) 2.0)))

(event Input|AxisEvents|InputAxisVertical
  (params (AxisValue :type Float%20%28single-precision%29))
  ;[1 1 1] Move player ship up and down using input
  (Variables|Default|SetCurrentPitchSpeed (Math|Interpolation|FInterpTo (Variables|Default|GetCurrentPitchSpeed) (+ (* AxisValue (Variables|Default|GetPlayerTurnSpeed) -1.0) (* (Math|Float|Absolute(Float) (Variables|Default|GetCurrentYawSpeed)) -0.5)) (Utilities|Time|GetWorldDeltaSeconds) 2.0)))

(event Input|AxisEvents|InputAxisAccelerate
  (params (AxisValue :type Float%20%28single-precision%29))
  (bind _acceleration (Variables|Default|GetAcceleration))
  ;[1 1 1] Accelerate the ship when enter key is held down
  (if (== AxisValue 1.0)
    (Components|Activation|SetActive (Variables|Default|GetThrustParticle) true false)
    (Audio|PlaySoundatLocation "/Game/Sounds/ThrusterSound.ThrusterSound" (Transformation|GetActorLocation) "0, 0, 0" 1.0 1.0 0.0 0 0 0)
    (else
      (Components|Activation|SetActive (Variables|Default|GetThrustParticle) false false)))
  (Variables|Default|SetCurrentPlayerSpeed (Math|Float|Clamp(Float) (+ (Variables|Default|GetCurrentPlayerSpeed) (* (Math|Float|SelectFloat (* AxisValue _acceleration) (* _acceleration -0.3) (!= AxisValue 0.0)) (Utilities|Time|GetWorldDeltaSeconds))) (Variables|Default|GetMinPlayerSpeed) (Variables|Default|GetMaxPlayerSpeed))))

(fn ConstructionScript)