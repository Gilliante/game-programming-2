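; Collectable pickup actor that decrements NumCollectables in MainGameState2, plays a sound and destroys itself when an actor tagged "player" overlaps it.
; Tick bobs it vertically and swings its yaw using sine differences added to the current transform.
; The bob uses DeltaSeconds, but the yaw uses a fixed offset, so its swing depends on frame rate.
; Particle spawn and Wait countdown nodes are disconnected and never run.
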(event EventBeginPlay)

(event Collision|EventActorBeginOverlap
  (params (OtherActor :type Actor%20Object%20Reference))
  ;[1 1 1] Check if overlapping with player. If so, change the number of collectables in scene and remove
  (if (Actor|ActorHasTag OtherActor "player")
    (bind _asmain_game_state_2 (Utilities|Casting|CastToMainGameState2 (Game|GetGameState)))
    (Variables|/Game/GameModes/MainGameState2.MainGameState2_C|SetNumCollectables _asmain_game_state_2 (+ (Variables|/Game/GameModes/MainGameState2.MainGameState2_C|GetNumCollectables _asmain_game_state_2) -1))
    (Audio|PlaySoundatLocation "/Game/Sounds/CollectSound.CollectSound" (Transformation|GetActorLocation) "0, 0, 0" 1.0 1.0 0.0 0 0 0)
    (Actor|DestroyActor)))

(event EventTick
  (params (DeltaSeconds :type Float%20%28single-precision%29))
  (bind _returnvalue (Actor|GetGameTimeSinceCreation))
  (bind _returnvalue_2 (Actor|GetGameTimeSinceCreation))
  (bind _returnvalue_3 (Transformation|GetActorRotation))
  (bind _returnvalue_4 (Transformation|GetActorLocation))
  (bind (_roll _pitch _yaw) (Math|Rotator|BreakRotator _returnvalue_3))
  (bind (_x _y _z) (Math|Vector|BreakVector _returnvalue_4))
  ;[1 1 1] Rotate back and forth and move the collectable up and down every tick using sin function
  (Transformation|SetActorRotation (Math|Rotator|MakeRotator _roll _pitch (+ _yaw (* (- (Math|Trig|Sin(Radians) (+ _returnvalue_2 1.0)) (Math|Trig|Sin(Radians) _returnvalue_2)) 8.0))))
  (Transformation|SetActorLocation (Math|Vector|MakeVector _x _y (+ _z (* (- (Math|Trig|Sin(Radians) (+ _returnvalue DeltaSeconds)) (Math|Trig|Sin(Radians) _returnvalue)) 8e+01))) false false))

(fn ConstructionScript)