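; Enemy projectile that damages the player and also destroys any enemy ship it overlaps.
; Tick accelerates it along negative local X per frame, reports IsHit to GameManager1_Blueprint, and destroys it at a speed threshold unless DestroyActor is set.
; Overlaps use actor tags, update health or enemy count through the level's game mode (MainGameMode or MainGameMode2), spawn effects, and set DestroyActor, which keeps Tick moving the bullet.
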(event EventBeginPlay)

(event EventTick
  (params (DeltaSeconds :type Float%20%28single-precision%29))
  ;[1 1 1] Move Bullet and destroy it once it get's to a certain distance
  (if (or (Math|Vector|NotEqual(Vector) (Variables|Default|GetBulletSpeed) "-900.000000,0.000000,0.000000" 0.0001) (Variables|Default|GetdestroyActor))
    (bind _output_get (Variables|Default|SetBulletSpeed (+ (Variables|Default|GetBulletSpeed) "-20.000000,0.000000,0.000000")))
    (Transformation|AddActorLocalOffset _output_get false false)
    (bind _outactors (Actor|GetAllActorswithTag "manager"))
    (bind _asgame_manager_1_blueprint (Utilities|Casting|CastToGameManager1_Blueprint (Utilities|Array|Get(acopy) _outactors)))
    (Class|GameManager|IsEnemyHit _asgame_manager_1_blueprint (Variables|Default|GetIsHit))
    (Class|GameManager|GetEnemyCount _asgame_manager_1_blueprint)
    (Variables|Default|SetIsHit false)
    (else
      (Actor|DestroyActor))))

(event Collision|EventActorBeginOverlap
  (params (OtherActor :type Actor%20Object%20Reference))
  (bind _returnvalue (Game|GetGameMode))
  (bind _returnvalue_2 (Game|GetGameMode))
  (bind _returnvalue_3 (Actor|ActorHasTag OtherActor "enemy"))
  ;[1 1 1] If colliding with player, change the player's health
  (Variables|Default|SetLocation (Transformation|GetActorLocation OtherActor))
  (if (Actor|ActorHasTag OtherActor "player")
    (Variables|Default|SetPlayerShip OtherActor)
    (bind _returnvalue_4 (Game|GetCurrentLevelName true))
    (if (Utilities|Enum|Equal(Enum) _returnvalue_4 "Level1")
      (bind _asmain_game_mode (Utilities|Casting|CastToMainGameMode _returnvalue))
      (Default|UpdatePlayerHealth _asmain_game_mode 15.0)
      (Audio|PlaySoundatLocation "/Game/Sounds/DestroySound.DestroySound" (Transformation|GetActorLocation (Game|Player|GetPlayerPawn 0)) "0, 0, 0" 1.0 1.0 0.0 0 0 0)
      (else
        (bind _asmain_game_mode_2 (Utilities|Casting|CastToMainGameMode2 _returnvalue))
        (Default|UpdatePlayerHealth _asmain_game_mode_2 15.0)
        (Audio|PlaySoundatLocation "/Game/Sounds/DestroySound.DestroySound" (Transformation|GetActorLocation (Game|Player|GetPlayerPawn 0)) "0, 0, 0" 1.0 1.0 0.0 0 0 0)))
    (Effects|SpawnEmitteratLocation "/Game/Particles/HitParticle.HitParticle" (Transformation|GetActorLocation (Game|Player|GetPlayerPawn 0)) "0, 0, 0" "5.000000,5.000000,5.000000")
    (Variables|Default|SetdestroyActor true)
    (else
      ;[1 1 1] If colliding with enemy, destroy them and change the enemy count
      (if _returnvalue_3
        (bind _output_get (Variables|Default|SetShipToDestroy OtherActor))
        (bind _output_get_2 (Variables|Default|SetIsHit _returnvalue_3))
        (if _output_get_2
          (Actor|DestroyActor _output_get)
          (bind _returnvalue_5 (Game|GetCurrentLevelName true))
          (if (Utilities|Enum|Equal(Enum) _returnvalue_5 "Level1")
            (bind _asmain_game_mode_2 (Utilities|Casting|CastToMainGameMode _returnvalue_2))
            (Default|UpdateEnemyCount _asmain_game_mode_2)
            (Effects|SpawnEmitteratLocation "/Game/Particles/DestroyParticle.DestroyParticle" (Variables|Default|GetLocation) "0, 0, 0" "2.000000,2.000000,2.000000")
            (Variables|Default|SetdestroyActor true)
            (else
              (bind _asmain_game_mode_2_2 (Utilities|Casting|CastToMainGameMode2 _returnvalue_2))
              (Default|UpdateEnemyCount _asmain_game_mode_2_2)
              (Effects|SpawnEmitteratLocation "/Game/Particles/DestroyParticle.DestroyParticle" (Variables|Default|GetLocation) "0, 0, 0" "2.000000,2.000000,2.000000")
              (Variables|Default|SetdestroyActor true))))))))

(fn ConstructionScript)