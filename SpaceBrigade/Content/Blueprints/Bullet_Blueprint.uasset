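; Bullet actor for a ship shooter that plays a shot sound on spawn and damages the player or enemy ships on overlap.
; Tick accelerates it along local Z without delta-time scaling, reports hits to the tagged GameManager1_Blueprint, and destroys it at a speed cap.
; Overlaps branch on actor tags: player hits update health via MainGameMode, enemies die instantly, and EnemyShip3 loses health.
; Kills update the level-specific game mode's enemy count and destroy the bullet.
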(event EventBeginPlay
  (Audio|PlaySoundatLocation "/Game/Sounds/ShootSound.ShootSound" (Transformation|GetActorLocation (Game|Player|GetPlayerPawn 0)) "0, 0, 0" 1.0 1.0 0.0 0 0 0))

(event EventTick
  (params (DeltaSeconds :type Float%20%28single-precision%29))
  ;[1 1 1] Move Bullet and destroy it once it get's to a certain distance
  (if (Math|Vector|NotEqual(Vector) (Variables|Default|GetBulletSpeed) "0, 0,600.000000" 0.0001)
    (bind _output_get (Variables|Default|SetBulletSpeed (+ (Variables|Default|GetBulletSpeed) "0, 0,20.000000")))
    (Transformation|AddActorLocalOffset _output_get false false)
    (bind _outactors (Actor|GetAllActorswithTag "manager"))
    (bind _asgame_manager_1_blueprint (Utilities|Casting|CastToGameManager1_Blueprint (Utilities|Array|Get(acopy) _outactors)))
    (Class|GameManager|IsEnemyHit _asgame_manager_1_blueprint (Variables|Default|GetIsHit))
    (Class|GameManager|GetEnemyCount _asgame_manager_1_blueprint)
    (Variables|Default|SetIsHit false)
    (else
      (Actor|DestroyActor))))

(event Collision|EventActorBeginOverlap
  (params (OtherActor :type Actor%20Object%20Reference))
  (bind _returnvalue (Game|GetGameMode))
  (bind _returnvalue_2 (Game|Player|GetPlayerPawn 0))
  (bind _returnvalue_3 (Game|GetGameMode))
  (bind _returnvalue_4 (Actor|ActorHasTag OtherActor "enemy"))
  (bind _returnvalue_5 (Transformation|GetActorLocation _returnvalue_2))
  ;[1 1 1] If colliding with player, change the player's health
  (Variables|Default|SetLocation (Transformation|GetActorLocation))
  (if (Actor|ActorHasTag OtherActor "player")
    (Variables|Default|SetPlayerShip OtherActor)
    (bind _asmain_game_mode (Utilities|Casting|CastToMainGameMode (Game|GetGameMode)))
    (Default|UpdatePlayerHealth _asmain_game_mode 15.0)
    (Audio|PlaySoundatLocation "/Game/Sounds/DestroySound.DestroySound" _returnvalue_5 "0, 0, 0" 1.0 1.0 0.0 0 0 0)
    (Effects|SpawnEmitteratLocation "/Game/Particles/DestroyParticle.DestroyParticle" _returnvalue_5 "0, 0, 0" "5.000000,5.000000,5.000000")
    (else
      ;[1 1 1] If colliding with enemy, destroy them and change the enemy count. If enemy colliding with is enemy3, then decrease it's health. If it's health reaches 0, destroy it
      (if _returnvalue_4
        (bind _output_get (Variables|Default|SetShipToDestroy OtherActor))
        (bind _output_get_2 (Variables|Default|SetIsHit _returnvalue_4))
        (if _output_get_2
          (Actor|DestroyActor _output_get)
          (Audio|PlaySoundatLocation "/Game/Sounds/DestroySound.DestroySound" (Variables|Default|GetLocation) "0, 0, 0" 1.0 1.0 0.0 0 0 0)
          (Effects|SpawnEmitteratLocation "/Game/Particles/DestroyParticle.DestroyParticle" (Variables|Default|GetLocation) "0, 0, 0" "5.000000,5.000000,5.000000")
          (bind _returnvalue_6 (Game|GetCurrentLevelName true))
          (if (Utilities|Enum|Equal(Enum) _returnvalue_6 "Level1")
            (bind _asmain_game_mode_2 (Utilities|Casting|CastToMainGameMode _returnvalue_3))
            (Default|UpdateEnemyCount _asmain_game_mode_2)
            (else
              (bind _asmain_game_mode_2 (Utilities|Casting|CastToMainGameMode2 _returnvalue_3))
              (Default|UpdateEnemyCount _asmain_game_mode_2)))
          (Actor|DestroyActor))
        (elif (Actor|ActorHasTag OtherActor "enemy3")
          (bind _output_get_3 (Variables|Default|SetShipToDestroy OtherActor))
          (bind _asenemy_ship_3 (Utilities|Casting|CastToEnemyShip3 _output_get_3))
          (if (<= (Variables|/Game/Blueprints/EnemyShip3.EnemyShip3_C|GetHealth _asenemy_ship_3) 0.0)
            (Actor|DestroyActor (Variables|Default|GetShipToDestroy))
            (Audio|PlaySoundatLocation "/Game/Sounds/DestroySound.DestroySound" (Variables|Default|GetLocation) "0, 0, 0" 1.0 1.0 0.0 0 0 0)
            (Effects|SpawnEmitteratLocation "/Game/Particles/DestroyParticle.DestroyParticle" (Variables|Default|GetLocation) "0, 0, 0" "5.000000,5.000000,5.000000")
            (bind _returnvalue_7 (Game|GetCurrentLevelName true))
            (if (Utilities|Enum|Equal(Enum) _returnvalue_7 "Level1")
              (bind _asmain_game_mode_3 (Utilities|Casting|CastToMainGameMode _returnvalue))
              (Default|UpdateEnemyCount _asmain_game_mode_3)
              (else
                (bind _asmain_game_mode_2_2 (Utilities|Casting|CastToMainGameMode2 _returnvalue))
                (Default|UpdateEnemyCount _asmain_game_mode_2_2)))
            (Actor|DestroyActor)
            (else
              (Variables|/Game/Blueprints/EnemyShip3.EnemyShip3_C|SetHealth _asenemy_ship_3 (- (Variables|/Game/Blueprints/EnemyShip3.EnemyShip3_C|GetHealth _asenemy_ship_3) 15.0))
              (Audio|PlaySoundatLocation "/Game/Sounds/DestroySound.DestroySound" (Variables|Default|GetLocation) "0, 0, 0" 1.0 1.0 0.0 0 0 0)
              (Effects|SpawnEmitteratLocation "/Game/Particles/HitParticle.HitParticle" (Variables|Default|GetLocation) "5.000000,5.000000,5.000000"))))))))

(fn ConstructionScript)