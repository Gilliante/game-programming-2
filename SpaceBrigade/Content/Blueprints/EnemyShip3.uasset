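; EnemyShip3 is an enemy ship that affects the player's health and plays a collapse sound when they overlap.
; On overlap with a "player"-tagged actor, it picks MainGameMode for Level1 or MainGameMode2 for other levels and calls UpdatePlayerHealth with a fixed amount.
; Its own Health is initialized on BeginPlay but is not otherwise used in this Blueprint.
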(event EventBeginPlay
  ;[1 1 1] Set enemy health
  (Variables|Default|SetHealth 1e+02))

(event Collision|EventActorBeginOverlap
  (params (OtherActor :type Actor%20Object%20Reference))
  ;[1 1 1] Check if overlapping with player. If so, change the player health
  (Variables|Default|SetPlayer OtherActor)
  (bind _output_get (Variables|Default|SetPlayerHit (Actor|ActorHasTag OtherActor "player")))
  (if _output_get
    (bind _returnvalue (Game|GetCurrentLevelName true))
    (if (Utilities|Enum|Equal(Enum) _returnvalue "Level1")
      (bind _asmain_game_mode (Utilities|Casting|CastToMainGameMode (Game|GetGameMode)))
      (Default|UpdatePlayerHealth _asmain_game_mode 25.0)
      (Audio|PlaySoundatLocation "/Game/StarterContent/Audio/Collapse_Cue.Collapse_Cue" (Transformation|GetActorLocation (Game|Player|GetPlayerPawn 0)) "0, 0, 0" 1.0 1.0 0.0 0 0 0)
      (else
        (bind _asmain_game_mode_2 (Utilities|Casting|CastToMainGameMode2 (Game|GetGameMode)))
        (Default|UpdatePlayerHealth _asmain_game_mode_2 25.0)
        (Audio|PlaySoundatLocation "/Game/StarterContent/Audio/Collapse_Cue.Collapse_Cue" (Transformation|GetActorLocation (Game|Player|GetPlayerPawn 0)) "0, 0, 0" 1.0 1.0 0.0 0 0 0)))))

(event EventTick
  (params (DeltaSeconds :type Float%20%28single-precision%29)))

(fn ConstructionScript)